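; Procedural room Blueprint that builds a rectangular perimeter of corners, walls and optional doors in the Construction Script, with no runtime logic.
; It derives four corner points from the X/Y wall counts and the segment dimensions in WallStru, then places corner static meshes.
; Each side can get one BP_door child actor with its own lock setting and clamped slot index.
; Wall child actors then fill every slot not taken by a door.
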(event EventBeginPlay)

(event Collision|EventActorBeginOverlap
  (params (OtherActor :type Actor%20Object%20Reference)))

(event EventTick
  (params (DeltaSeconds :type Float%20%28single-precision%29)))

(fn ConstructionScript
  (bind _wall_stru (Variables|Default|Getwall_stru))
  (bind (_wall_width _wall_length) (Utilities|Struct|Breakwall_struct _wall_stru))
  (Variables|Default|Setwall_width _wall_width)
  (Variables|Default|Setwall_length _wall_length)
  (CallFunction|FUCFourPostion)
  (CallFunction|FUCSetFourConer)
  (CallFunction|FUCSetDoor)
  (CallFunction|FUCSetWall))

(fn FUCFourPostion
  (bind _y_wall_count (Variables|Default|GetY_wall_count))
  (bind _left_up_position (Variables|base|Getleft_up_position))
  (bind _wall_length (Variables|Default|Getwall_length))
  (bind _x_wall_count (Variables|Default|GetX_wall_count))
  (bind _wall_length_2 (Variables|Default|Getwall_length))
  (bind _returnvalue (+ _y_wall_count 2))
  (bind _returnvalue_2 (+ _x_wall_count 2))
  (bind _returnvalue_3 (* _returnvalue _wall_length))
  (bind _returnvalue_4 (* _returnvalue_2 _wall_length_2))
  ;[1 1 1] set four con location  设置四个基点的位置
  (Variables|base|Setright_up_position (Math|Vector|MakeVector (+ (.x _left_up_position) _returnvalue_4) (.y _left_up_position) (.z _left_up_position)))
  (Variables|base|Setleft_down_position (Math|Vector|MakeVector (.x _left_up_position) _returnvalue_3 (.z _left_up_position)))
  (Variables|base|Setright_down_position (Math|Vector|MakeVector _returnvalue_4 _returnvalue_3 (.z _left_up_position))))

(fn FUCSetFourConer
  (bind _right_down_position (Variables|base|Getright_down_position))
  (bind _left_up_position (Variables|base|Getleft_up_position))
  (bind _right_up_position (Variables|base|Getright_up_position))
  (bind _left_down_position (Variables|base|Getleft_down_position))
  ;[1 1 1] 生成四个墙角
  (AddComponent|AddStaticMeshComponent false (Math|Transform|MakeTransform (Math|Vector|MakeVector (+ (.x _left_up_position) (Variables|Default|Getwall_length)) (.y _left_up_position) (.z _left_up_position)) "0,180.000000, 0" "1,1,1"))
  (AddComponent|AddStaticMeshComponent false (Math|Transform|MakeTransform (Math|Vector|MakeVector (.x _right_up_position) (+ (.y _right_up_position) (Variables|Default|Getwall_length)) (.z _right_up_position)) "0,-90.000000, 0" "1,1,1"))
  (AddComponent|AddStaticMeshComponent false (Math|Transform|MakeTransform (Math|Vector|MakeVector (.x _left_down_position) (- (.y _left_down_position) (Variables|Default|Getwall_length)) (.z _left_down_position)) "0,90.000000, 0" "1,1,1"))
  (AddComponent|AddStaticMeshComponent false (Math|Transform|MakeTransform (Math|Vector|MakeVector (- (.x _right_down_position) (Variables|Default|Getwall_length)) (.y _right_down_position) (.z _right_down_position)) "0, 0, 0" "1,1,1")))

(fn FUCSetWall
  (bind _wall_length (Variables|Default|Getwall_length))
  (bind _left_up_position (Variables|base|Getleft_up_position))
  (bind _wall_length_2 (Variables|Default|Getwall_length))
  (bind _left_up_position_2 (Variables|base|Getleft_up_position))
  (bind _left_down_position (Variables|base|Getleft_down_position))
  (bind _right_up_position (Variables|base|Getright_up_position))
  (bind _door_down_count (Variables|door|Getdoor_down_count))
  (bind _door_left_count (Variables|door|Getdoor_left_count))
  (bind _door_right_count (Variables|door|Getdoor_right_count))
  ;[1 1 1] X方向上的墙体
  (for _index (range 0 (- (Variables|Default|GetX_wall_count) 1))
    (if (not (== (Variables|door|Getdoor_up_count) (+ _index 1)))
      (bind _returnvalue (AddComponent|AddChildActorComponent false (Math|Transform|MakeTransform (Math|Vector|MakeVector (+ (.x _left_up_position) (* (+ _index 1) _wall_length_2) _wall_length_2) (.y _left_up_position) (.z _left_up_position)) "0,180.000000, 0" "1,1,1")))
      (Utilities|Array|Add (Variables|Default|GetWall) _returnvalue)))
  (for _index_2 (range 0 (- (Variables|Default|GetX_wall_count) 1))
    (if (not (and (> _door_down_count 0) (== _door_down_count (+ _index_2 1))))
      (bind _returnvalue_2 (AddComponent|AddChildActorComponent false (Math|Transform|MakeTransform (Math|Vector|MakeVector (+ (.x _left_down_position) (* (+ _index_2 1) (Variables|Default|Getwall_length))) (.y _left_down_position) (.z _left_down_position)) "0, 0, 0" "1,1,1")))
      (Utilities|Array|Add (Variables|Default|GetWall) _returnvalue_2)))
  ;[1 1 1] Y 方向的墙体
  (for _index_3 (range 0 (- (Variables|Default|GetY_wall_count) 1))
    (if (not (and (> _door_left_count 0) (== _door_left_count (+ _index_3 1))))
      (bind _returnvalue_3 (AddComponent|AddChildActorComponent false (Math|Transform|MakeTransform (Math|Vector|MakeVector (.x _left_up_position_2) (+ (* (+ _index_3 1) (Variables|Default|Getwall_length)) (.y _left_up_position_2) 0.0) (.z _left_up_position_2)) "0,90.000000, 0" "1,1,1")))
      (Utilities|Array|Add (Variables|Default|GetWall) _returnvalue_3)))
  (for _index_4 (range 0 (- (Variables|Default|GetY_wall_count) 1))
    (if (not (and (> _door_right_count 0) (== _door_right_count (+ _index_4 1))))
      (bind _returnvalue_4 (AddComponent|AddChildActorComponent false (Math|Transform|MakeTransform (Math|Vector|MakeVector (.x _right_up_position) (+ (* (+ _index_4 1) _wall_length) (.y _right_up_position) _wall_length) (.z _right_up_position)) "0,-90.000000, 0" "1,1,1")))
      (Utilities|Array|Add (Variables|Default|GetWall) _returnvalue_4))))

(fn FUCSetDoor
  (bind _left_up_position (Variables|base|Getleft_up_position))
  (bind _left_up_position_2 (Variables|base|Getleft_up_position))
  (bind _wall_length (Variables|Default|Getwall_length))
  (bind _wall_length_2 (Variables|Default|Getwall_length))
  (bind _left_down_position (Variables|base|Getleft_down_position))
  (bind _right_up_position (Variables|base|Getright_up_position))
  ;[1 1 1] X 方向上的门
  (if (> (Variables|door|Getdoor_up_count) 0)
    (bind _returnvalue (AddComponent|AddChildActorComponent false (Math|Transform|MakeTransform (Math|Vector|MakeVector (+ (.x _left_up_position) (* (Math|Integer|Clamp(Integer) (Variables|door|Getdoor_up_count) 1 (Variables|Default|GetX_wall_count)) (Variables|Default|Getwall_length))) (+ (.y _left_up_position) (Variables|Default|Getwall_width)) (.z _left_up_position)) "0, 0, 0" "1,1,1")))
    (bind _asbp_door (Utilities|Casting|CastToBP_door (Variables|/Script/Engine.ChildActorComponent|GetChildActor _returnvalue)))
    (Variables|/Game/Light/BluePrint/common/BP_door.BP_door_C|SetLock? _asbp_door (Variables|Default|Gettop_door_lock?))
    (Variables|door|Setdoor_up_count (Math|Integer|Clamp(Integer) (Variables|door|Getdoor_up_count) 1 (Variables|Default|GetX_wall_count))))
  (if (> (Variables|door|Getdoor_down_count) 0)
    (bind _returnvalue_2 (AddComponent|AddChildActorComponent false (Math|Transform|MakeTransform (Math|Vector|MakeVector (+ (.x _left_down_position) (* (Math|Integer|Clamp(Integer) (Variables|door|Getdoor_down_count) 1 (Variables|Default|GetX_wall_count)) _wall_length_2) _wall_length_2) (- (.y _left_down_position) (Variables|Default|Getwall_width)) (.z _left_down_position)) "0,180.000000, 0" "1,1,1")))
    (bind _asbp_door_2 (Utilities|Casting|CastToBP_door (Variables|/Script/Engine.ChildActorComponent|GetChildActor _returnvalue_2)))
    (Variables|/Game/Light/BluePrint/common/BP_door.BP_door_C|SetLock? _asbp_door_2 (Variables|Default|Getdown_door_lock?))
    (Variables|door|Setdoor_down_count (Math|Integer|Clamp(Integer) (Variables|door|Getdoor_down_count) 1 (Variables|Default|GetX_wall_count))))
  ;[1 1 1] Y方向上的门
  (if (> (Variables|door|Getdoor_left_count) 0)
    (bind _returnvalue_3 (AddComponent|AddChildActorComponent false (Math|Transform|MakeTransform (Math|Vector|MakeVector (+ (.x _left_up_position_2) (Variables|Default|Getwall_width)) (+ (.y _left_up_position_2) (* (Math|Integer|Clamp(Integer) (Variables|door|Getdoor_left_count) 1 (Variables|Default|GetY_wall_count)) _wall_length) _wall_length) (.z _left_up_position_2)) "0,-90.000000, 0" "1,1,1")))
    (bind _asbp_door_3 (Utilities|Casting|CastToBP_door (Variables|/Script/Engine.ChildActorComponent|GetChildActor _returnvalue_3)))
    (Variables|/Game/Light/BluePrint/common/BP_door.BP_door_C|SetLock? _asbp_door_3 (Variables|Default|Getleft_door_lock?))
    (Variables|door|Setdoor_left_count (Math|Integer|Clamp(Integer) (Variables|door|Getdoor_left_count) 1 (Variables|Default|GetY_wall_count))))
  (if (> (Variables|door|Getdoor_right_count) 0)
    (bind _returnvalue_4 (AddComponent|AddChildActorComponent false (Math|Transform|MakeTransform (Math|Vector|MakeVector (- (.x _right_up_position) (Variables|Default|Getwall_width)) (+ (.y _right_up_position) (* (Math|Integer|Clamp(Integer) (Variables|door|Getdoor_right_count) 1 (Variables|Default|GetX_wall_count)) (Variables|Default|Getwall_length))) (.z _right_up_position)) "0,90.000000, 0" "1,1,1")))
    (bind _asbp_door_4 (Utilities|Casting|CastToBP_door (Variables|/Script/Engine.ChildActorComponent|GetChildActor _returnvalue_4)))
    (Variables|/Game/Light/BluePrint/common/BP_door.BP_door_C|SetLock? _asbp_door_4 (Variables|Default|Getright_door_lock?))
    (Variables|door|Setdoor_right_count (Math|Integer|Clamp(Integer) (Variables|door|Getdoor_right_count) 1 (Variables|Default|GetX_wall_count)))))