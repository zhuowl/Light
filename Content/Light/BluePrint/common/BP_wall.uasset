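; BP_wall is a breakable wall that lets light from BP_mainLight actors through once damage opens a hole.
; Overlap with the player girl's box toggles a material highlight and decal while it is intact.
; When hardness runs out, it swaps in a holed mesh and tells BP_manager to update lighting.
; For each main light whose line trace hits the wall, it spawns a BP_Light laser continuing away from that source.
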(event OnComponentBeginOverlap(Box)
  (params (OverlappedComponent :type Primitive%20Component%20Object%20Reference) (OtherActor :type Actor%20Object%20Reference) (OtherComp :type Primitive%20Component%20Object%20Reference) (OtherBodyIndex :type Integer) (bFromSweep :type Boolean) (SweepResult :type Hit%20Result%20Structure%20%28by%20ref%29))
  (bind (_asbp_character_girl _bsuccess) (Utilities|Casting|CastToBP_character_girl OtherActor))
  (if (and _bsuccess (not (Variables|Default|Gethas_holes)))
    (if (== OtherComp (Variables|/Game/Light/BluePrint/character/BP_character_girl.BP_character_girl_C|GetBox _asbp_character_girl))
      (Rendering|Material|SetScalarParameterValueonMaterials (Variables|Default|GetSM_wall) "control" 1.0)
      (Rendering|SetVisibility (Variables|Default|GetDecal) true false))))

(event OnComponentEndOverlap(Box)
  (params (OverlappedComponent :type Primitive%20Component%20Object%20Reference) (OtherActor :type Actor%20Object%20Reference) (OtherComp :type Primitive%20Component%20Object%20Reference) (OtherBodyIndex :type Integer))
  (if (not (Variables|Default|Gethas_holes))
    (if (.bSuccess (Utilities|Casting|CastToBP_character_girl OtherActor))
      (Rendering|Material|SetScalarParameterValueonMaterials (Variables|Default|GetSM_wall) "control" 0.0)
      (Rendering|SetVisibility (Variables|Default|GetDecal) false false))))

(event Custom|spawn_Light
  (params (main_Light :type Actor%20Object%20Reference))
  (bind _returnvalue (Transformation|GetActorLocation main_Light))
  (bind _scene (Variables|Default|GetScene))
  (bind _returnvalue_2 (Transformation|GetWorldLocation _scene))
  (bind _returnvalue_3 (- _returnvalue_2 _returnvalue))
  (bind _returnvalue_4 (Math|Vector|Normalize _returnvalue_3))
  (bind _returnvalue_5 (* _returnvalue_4 1e+02))
  (bind _returnvalue_6 (+ _returnvalue_5 _returnvalue_2))
  ;[1 1 1] spawn_light
  (bind _returnvalue_7 (Game|SpawnActorfromClass "/Game/Light/BluePrint/common/BP_Light.BP_Light_C" (Transformation|GetWorldTransform _scene) "Undefined" 0 0))
  (Utilities|Array|Add (Variables|Default|Getlight) _returnvalue_7)
  (Default|SpawnLaser _returnvalue_7 _returnvalue_2 (Math|Vector|MakeVector (.x _returnvalue_6) (.y _returnvalue_6) (.z (Transformation|GetWorldLocation _scene)))))

(event Custom|main_light_influence
  (params (MainLight :type Actor%20Object%20Reference))
  ;[1 1 1] 主光源的影响
  (bind _can_get_mainlight (CallFunction|FUCCanMainLightLight MainLight))
  (if _can_get_mainlight
    (CallFunction|SpawnLight MainLight)))

(event Custom|change_to_hole
  ;[1 1 1] 改变状态为，已有洞
  (Components|DestroyComponent (Variables|Default|GetSM_wall))
  (bind _returnvalue (AddComponent|AddStaticMeshComponent false))
  (Components|StaticMesh|SetStaticMesh _returnvalue (Variables|Default|Getholes_wall))
  (Default|UpdateLight (Variables|Default|Getmanger)))

(event EventBeginPlay
  ;[1 1 1] begin
  (bind _outactors (Actor|GetAllActorsOfClass "/Game/Light/BluePrint/common/BP_mainLight.BP_mainLight_C"))
  (Variables|Default|Setmain_light _outactors)
  (bind _outactors_2 (Actor|GetAllActorsOfClass "/Game/Light/BluePrint/Game/BP_manager.BP_manager_C"))
  (Variables|Default|Setmanger (Utilities|Array|Get(acopy) _outactors_2)))

(event Collision|EventActorBeginOverlap
  (params (OtherActor :type Actor%20Object%20Reference)))

(event Game|Damage|EventAnyDamage
  (params (Damage :type Float%20%28single-precision%29) (DamageType :type Damage%20Type%20Object%20Reference) (InstigatedBy :type Controller%20Object%20Reference) (DamageCauser :type Actor%20Object%20Reference))
  ;[1 1 1] take damage
  (Variables|Default|Sethardness (- (Variables|Default|Gethardness) Damage))
  ;[1 1 1] tcik
  (if (<= (Variables|Default|Gethardness) 0.0)
    (Variables|Default|Sethas_holes true)
    (Utilities|FlowControl|DoOnce false
      (:Completed
        (CallFunction|ChangetoHole)
        (Utilities|FlowControl|Delay 0.1)
        (for _array_element (Variables|Default|Getmain_light)
          (CallFunction|MainLightInfluence _array_element))))))

(fn ConstructionScript)

(fn FUCCanMainLightLight
  (params (MainLight :type Actor%20Object%20Reference))
  (bind _returnvalue (Transformation|GetActorLocation MainLight))
  (bind _outhit (Collision|LineTraceByChannel _returnvalue (+ _returnvalue (* (Math|Vector|Normalize (- (Transformation|GetWorldLocation (Variables|Default|GetScene)) _returnvalue)) 1e+03)) "TraceTypeQuery2" true 0 "ForDuration" false))
  (return (Utilities|Enum|Equal(Enum) (Utilities|GetDisplayName (.HitActor (Collision|BreakHitResult _outhit))) (Utilities|GetDisplayName self))))