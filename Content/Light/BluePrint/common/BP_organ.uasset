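; BP_organ is a mechanism actor that keeps a referenced door locked until it is triggered.
; On BeginPlay it caches the first BP_manager in the level and locks its ControlDoor.
; The open_control_door event unlocks a valid door on each call and opens it through a DoOnce, so the opening runs only once.
; Nothing in this graph calls that event or uses the cached manager.
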(event Custom|open_control_door
  (bind _control_door (Variables|Default|Getcontrol_Door))
  (Utilities|IsValid _control_door
    (:Is%20Valid
      (Variables|/Game/Light/BluePrint/common/BP_door.BP_door_C|SetLock? _control_door false)
      (Utilities|FlowControl|DoOnce false
        (:Completed
          (Default|DoorOpen _control_door))))))

(event EventBeginPlay
  (bind _outactors (Actor|GetAllActorsOfClass "/Game/Light/BluePrint/Game/BP_manager.BP_manager_C"))
  (Variables|Default|Setmanger (Utilities|Array|Get(acopy) _outactors))
  (Variables|/Game/Light/BluePrint/common/BP_door.BP_door_C|SetLock? (Variables|Default|Getcontrol_Door) true))

(event Collision|EventActorBeginOverlap
  (params (OtherActor :type Actor%20Object%20Reference)))

(event EventTick
  (params (DeltaSeconds :type Float%20%28single-precision%29)))

(fn ConstructionScript)