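; BP_startPawn is a pawn whose only working behavior is opening Light_level_01 when Gamepad Special Right is pressed.
; The level opens directly by name from the key event, and the turn axis events, BeginPlay and construction script are empty.
; Unconnected leftover nodes hold clamped mouse and rate-scaled yaw input, plus a forward line trace that casts to BP_character_girl, none of which runs.
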(event EventBeginPlay)

(event Collision|EventActorBeginOverlap
  (params (OtherActor :type Actor%20Object%20Reference)))

(event EventTick
  (params (DeltaSeconds :type Float%20%28single-precision%29)))

(event Input|AxisEvents|InputAxisTurnRate
  (params (AxisValue :type Float%20%28single-precision%29))
  ;[1 1 1] Gamepad_input
)

(event Input|AxisEvents|InputAxisTurn
  (params (AxisValue :type Float%20%28single-precision%29))
  ;[1 1 1] Mouse_input
)

(event Input|GamepadEvents|GamepadSpecialRight
  (params (Key :type Key%20Structure))
  (:Pressed
    (Game|OpenLevel(byName) "Light_level_01")))

(fn ConstructionScript)