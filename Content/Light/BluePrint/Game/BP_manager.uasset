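; BP_manager is the game manager actor for a light puzzle game, handling light updates, hints, pausing and game over.
; Its events refresh laser lists on every BP_Light and pass a new main light to each BP_wall with holes.
; It creates hint and pause widgets at BeginPlay, flashes the magnifier hint, and toggles pause via FlipFlop from Enter or gamepad.
; GameOver triggers the girl character's win or fail, then shows the result screen after a delay.
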(event Custom|update_light
  ;[1 1 1] 更新光线
  (bind _outactors (Actor|GetAllActorsOfClass "/Game/Light/BluePrint/common/BP_Light.BP_Light_C"))
  (for _array_element _outactors
    (Default|UpdateLaserList _array_element)))

(event Custom|GameOver
  (params (Win :type Boolean))
  (bind _returnvalue (Game|GetPlayerController 0))
  (bind _player (Variables|Default|GetPlayer))
  ;[1 1 1] GameOver  游戏结束
  (if Win
    (bind _returnvalue_2 (UserInterface|CreateWidget "/Game/Light/UI/UMG_win.UMG_win_C"))
    (bind _output_get (Variables|Default|SetUI_win _returnvalue_2))
    (Input|SetInputModeUIOnly _returnvalue _output_get "LockAlways")
    (Default|Win _player)
    (Utilities|FlowControl|Delay 1.5)
    (UserInterface|Viewport|AddtoViewport _output_get 0)
    (else
      (bind _returnvalue_3 (UserInterface|CreateWidget "/Game/Light/UI/UMG_lose.UMG_lose_C"))
      (bind _output_get_2 (Variables|Default|SetUI_lose _returnvalue_3))
      (Input|SetInputModeUIOnly _returnvalue _output_get_2 "LockAlways")
      (Default|Fail _player)
      (Utilities|FlowControl|Delay 1.5)
      (UserInterface|Viewport|AddtoViewport _output_get_2 0)))
  (Variables|/Script/Engine.PlayerController|SetbShowMouseCursor _returnvalue true))

(event Custom|call_needLopue_hint
  (bind _ui_needloupe_hint (Variables|Default|GetUI_needLoupe_hint))
  ;[1 1 1] 需要放大镜的提示
  (Widget|SetVisibility _ui_needloupe_hint "Visible")
  (Utilities|FlowControl|Delay 2.0)
  (Widget|SetVisibility _ui_needloupe_hint "Collapsed"))

(event Custom|pause
  (bind _returnvalue (Game|GetPlayerController 0))
  (bind _ui_pause (Variables|Default|GetUI_pause))
  ;[1 1 1] 按键控制  暂停
  (bind _isa (Utilities|FlowControl|FlipFlop)
    (:A
      (Game|SetGamePaused _isa)
      (UserInterface|Viewport|AddtoViewport _ui_pause 0)
      (Input|SetInputModeGameandUI _returnvalue _ui_pause "LockAlways" true)
      (Variables|/Script/Engine.PlayerController|SetbShowMouseCursor _returnvalue _isa))
    (:B
      (Game|SetGamePaused _isa)
      (Widget|RemovefromParent _ui_pause)
      (Input|SetInputModeGameOnly _returnvalue)
      (Variables|/Script/Engine.PlayerController|SetbShowMouseCursor _returnvalue _isa))))

(event Custom|add_mainLight
  (params (main_light :type BP%20Main%20Light%20Object%20Reference))
  ;[1 1 1] 增加主光源
  (bind _outactors (Actor|GetAllActorsOfClass "/Game/Light/BluePrint/common/BP_wall.BP_wall_C"))
  (for _array_element _outactors
    (if (Variables|/Game/Light/BluePrint/common/BP_wall.BP_wall_C|Gethas_holes _array_element)
      (Default|MainLightInfluence _array_element main_light))))

(event EventBeginPlay
  (Utilities|FlowControl|Sequence
    (:then_0
      (bind _returnvalue (UserInterface|CreateWidget "/Game/Light/UI/HInt/UMG_hint_needLoupe.UMG_hint_needLoupe_C"))
      (Variables|Default|SetUI_needLoupe_hint _returnvalue)
      (bind _returnvalue_2 (UserInterface|CreateWidget "/Game/Light/UI/HInt/UMG_hint_doorOpen.UMG_hint_doorOpen_C"))
      (Variables|Default|SetUI_doorOpen_hint _returnvalue_2)
      (bind _returnvalue_3 (UserInterface|CreateWidget "/Game/Light/UI/UMG_pause.UMG_pause_C"))
      (Variables|Default|SetUI_pause _returnvalue_3))
    (:then_1
      (bind _asbp_character_girl (Utilities|Casting|CastToBP_character_girl (Game|Player|GetPlayerPawn 0)))
      (Variables|Default|SetPlayer _asbp_character_girl))))

(event Collision|EventActorBeginOverlap
  (params (OtherActor :type Actor%20Object%20Reference)))

(event EventTick
  (params (DeltaSeconds :type Float%20%28single-precision%29)))

(event Input|KeyboardEvents|Enter
  (params (Key :type Key%20Structure))
  ;[1 1 1] 按键控制  暂停
  (:Pressed
    (CallFunction|Pause)))

(event Input|GamepadEvents|GamepadSpecialRight
  (params (Key :type Key%20Structure))
  ;[1 1 1] 按键控制  暂停
  (:Pressed
    (CallFunction|Pause)))

(fn ConstructionScript)